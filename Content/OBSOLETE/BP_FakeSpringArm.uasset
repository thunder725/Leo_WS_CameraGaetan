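; An actor that imitates a spring arm, positioning a camera behind a target it follows, with no collision check.
; Each tick, while the target is valid, it eases the camera toward an arm-length offset rotated by the actor's rotation.
; Only when UseControlRotation is set, it also turns from axis input with clamped pitch and interpolates its location toward the target plus an offset.
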(event EventTick
  (params (DeltaSeconds :type Float%20%28single-precision%29))
  (Variables|Following|GetTarget
    (:then
      (CallFunction|SetCameraTransform)
      (if (Variables|GeneralRotationParameters|GetUse%20Control%20Rotation)
        (CallFunction|Rotate)
        (CallFunction|FollowTarget)))
    (:else)))

(fn ConstructionScript)

(fn Rotate
  (Variables|Rotation|SetCurrent%20Yaw (+ (Variables|Rotation|GetCurrent%20Yaw) (* (Class|Actor|GetInputAxisKeyValue) (Variables|GeneralRotationParameters|GetMouse%20Sensitivity) (Utilities|Time|GetWorldDeltaSeconds))))
  (Variables|Rotation|SetCurrent%20Pitch (Math|Float|Clamp(Float) (+ (Variables|Rotation|GetCurrent%20Pitch) (* (Class|Actor|GetInputAxisKeyValue) (Variables|GeneralRotationParameters|GetMouse%20Sensitivity) (Utilities|Time|GetWorldDeltaSeconds))) -89.9999 89.9999))
  (Transformation|SetActorRotation (Math|Rotator|MakeRotator 0.0 (Variables|Rotation|GetCurrent%20Pitch) (Variables|Rotation|GetCurrent%20Yaw))))

(fn FollowTarget
  (Transformation|SetActorLocation (Math|Interpolation|VInterpTo (Transformation|GetActorLocation) (+ (Transformation|GetActorLocation (Variables|Following|GetTarget)) (Variables|Following|GetTarget%20Offset)) (Utilities|Time|GetWorldDeltaSeconds) (Variables|Following|GetMovement%20Smooth%20Time)) false false))

(fn SetCameraTransform
  (bind _camera (Variables|Default|GetCamera))
  (Transformation|SetWorldLocation _camera (Math|Interpolation|VInterpTo (Transformation|GetWorldLocation _camera) (+ (Transformation|GetActorLocation) (* (Transformation|GetActorRotation) (- (Variables|SpringArm|GetCameraOffset) (Math|Vector|MakeVector (Variables|SpringArm|GetSpring%20Arm%20Length) 0.0 0.0)))) (Utilities|Time|GetWorldDeltaSeconds) 1.0) false false))