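; BP_InteractableObjetc is an interactable actor that registers itself with the player character, BP_RWQFSFASXC, or both, as selected by InteractionType.
; Overlapping CollisionTrigger casts the other actor and sets its CurrentInteractable to this object.
; Ending the overlap clears that reference without checking whether it still points here, and both events print debug strings.
; OnInteract is an empty function, with no interaction logic in this Blueprint.
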(event OnComponentBeginOverlap(CollisionTrigger)
  (params (OverlappedComponent :type Primitive%20Component%20Object%20Reference) (OtherActor :type Actor%20Object%20Reference) (OtherComp :type Primitive%20Component%20Object%20Reference) (OtherBodyIndex :type Integer) (bFromSweep :type Boolean) (SweepResult :type Hit%20Result%20Structure%20%28by%20ref%29))
  (switch Utilities|FlowControl|Switch|SwitchonENUM_InteractableType (Variables|Default|GetInteractionType)
    (:NewEnumerator0
      (bind _asbp_main_character_character (Utilities|Casting|CastToBP_MainCharacter_Character OtherActor :!label _label))
      (Variables|/Game/ProjectSpeedbreaker/BPs/BP_MainCharacter_Character.BP_MainCharacter_Character_C|SetCurrentInteractable _asbp_main_character_character self)
      (Development|PrintString "Hello"))
    (:NewEnumerator1
      (bind _asbp_rwqfsfasxc (Utilities|Casting|CastToBP_RWQFSFASXC OtherActor :!label _label_2))
      (Variables|/Game/ProjectSpeedbreaker/BPs/BP_RWQFSFASXC.BP_RWQFSFASXC_C|SetCurrentInteractable _asbp_rwqfsfasxc self)
      (Development|PrintString "Hello" true true "(R=0.108543,G=1.000000,B=0.040252,A=1.000000)"))
    (:NewEnumerator2
      (Utilities|FlowControl|Sequence
        (:then_0
          (goto _label))
        (:then_1
          (goto _label_2))))))

(event OnComponentEndOverlap(CollisionTrigger)
  (params (OverlappedComponent :type Primitive%20Component%20Object%20Reference) (OtherActor :type Actor%20Object%20Reference) (OtherComp :type Primitive%20Component%20Object%20Reference) (OtherBodyIndex :type Integer))
  (switch Utilities|FlowControl|Switch|SwitchonENUM_InteractableType (Variables|Default|GetInteractionType)
    (:NewEnumerator0
      (bind _asbp_main_character_character (Utilities|Casting|CastToBP_MainCharacter_Character OtherActor :!label _label))
      (Variables|/Game/ProjectSpeedbreaker/BPs/BP_MainCharacter_Character.BP_MainCharacter_Character_C|SetCurrentInteractable _asbp_main_character_character 0)
      (Development|PrintString "Hello" true true "(R=1.000000,G=0.011239,B=0.809113,A=1.000000)"))
    (:NewEnumerator1
      (bind _asbp_rwqfsfasxc (Utilities|Casting|CastToBP_RWQFSFASXC OtherActor :!label _label_2))
      (Variables|/Game/ProjectSpeedbreaker/BPs/BP_RWQFSFASXC.BP_RWQFSFASXC_C|SetCurrentInteractable _asbp_rwqfsfasxc 0)
      (Development|PrintString "Hello" true true "(R=1.000000,G=0.694879,B=0.260123,A=1.000000)"))
    (:NewEnumerator2
      (Utilities|FlowControl|Sequence
        (:then_0
          (goto _label))
        (:then_1
          (goto _label_2))))))

(fn ConstructionScript)

(fn OnInteract)