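; BP_Interact_Move is an interactable that slides its static mesh along a set direction when interacted with.
; OnInteract sets a flag that lets Tick apply a frame-rate-scaled local offset, without sweep.
; A DoOnce-gated Delay clears the flag after TimeToGetThere as a makeshift timer.
; The DoOnce never resets, so only the first move gets timed.
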(event EventTick
  (params (DeltaSeconds :type Float%20%28single-precision%29))
  (if (Variables|Default|GetshouldMove)
    (Utilities|FlowControl|Sequence
      (:then_0
        ;[0.6314 1 0.3424] Make fakeTimer
        (Utilities|FlowControl|DoOnce false
          (:Completed
            (Utilities|FlowControl|Delay (Variables|Default|GetTimeToGetThere))
            (Variables|Default|SetshouldMove false))))
      (:then_1
        ;[1 0.204 0.8291] Actual Movement
        (Transformation|AddLocalOffset (Variables|Default|GetStaticMesh) (* (Variables|Default|GetDirectionToMove) DeltaSeconds 5e+01) false false)))))

(fn ConstructionScript
  (|CallParentFunction))

(fn OnInteract
  (Variables|Default|SetshouldMove true))